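; Fear is a short-lived actor that spawns one random fear manifestation and repels a Target.
; On BeginPlay it picks among FailedTest, Heights, DarkCloud and PeopleLaughingBP, spawns it at its own location, then destroys itself after a short delay.
; While alive, every Tick applies a linear-falloff radial force to the Target's Root, pushing it away from the actor.
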(event EventBeginPlay
  (bind _defaultsceneroot (Variables|Default|GetDefaultSceneRoot))
  (bind _returnvalue (Transformation|GetWorldLocation _defaultsceneroot))
  (bind _returnvalue_2 (Math|Transform|MakeTransform _returnvalue))
  (switch int (Math|Random|RandomIntegerinRange 0 3)
    (:0
      (Game|SpawnActorfromClass "/Game/Blueprints/Fears/FailedTest.FailedTest_C" _returnvalue_2 "AlwaysSpawn" 0 0))
    (:1
      (Game|SpawnActorfromClass "/Game/Blueprints/Fears/Heights.Heights_C" _returnvalue_2 "AlwaysSpawn" 0 0))
    (:2
      (Game|SpawnActorfromClass "/Game/Blueprints/Fears/DarkCloud.DarkCloud_C" _returnvalue_2 "AlwaysSpawn" 0 0))
    (:3
      (Game|SpawnActorfromClass "/Game/Blueprints/Fears/PeopleLaughingBP.PeopleLaughingBP_C" _returnvalue_2 "AlwaysSpawn" 0 0)))
  (Utilities|FlowControl|Delay 4.0)
  (Actor|DestroyActor))

(event Collision|EventActorBeginOverlap
  (params (OtherActor :type Actor%20Object%20Reference)))

(event EventTick
  (params (DeltaSeconds :type Float%20%28single-precision%29))
  (Physics|AddRadialForce (Variables|/Game/Blueprints/Target.Target_C|GetRoot (Variables|Default|GetTarget)) (Transformation|GetWorldLocation (Variables|Default|GetDefaultSceneRoot)) 1e+04 6.75e+03 "RIF_Linear" false))

(fn ConstructionScript)